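; Player character Blueprint that adds procedural camera motion for shooting, aiming, sprinting, reloading, melee, grenade and ultimate actions.
; Start/End events drive Timelines that move the camera, arms or spring arm and change FOV, with several rotations offset from CameraRotationWithPawn and pawn control rotation toggled around them.
; It also creates the HUD widget, deactivates particle systems on BeginPlay and toggles scope visibility.
; Death only prints a placeholder message, and some End events are empty.
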(event `self.ReceiveTick`
  (params (DeltaSeconds :type "Float (single-precision)")))

(event `self.ReceiveBeginPlay`
  ;[1 1 1] Begin PLay
  (bind _returnvalue (`|CreateWidget` "/Game/Character/TemporalMainWidget1.TemporalMainWidget1_C"))
  (`UserWidget.AddToPlayerScreen` _returnvalue 0)
  (`ActorComponent.Deactivate` (`self.ParticleSystem2`))
  (`ActorComponent.Deactivate` (`self.ParticleSystem`))
  (`ActorComponent.Deactivate` (`self.ParticleSystem3`))
  (`ActorComponent.Deactivate` (`self.ParticleSystem1`)))

(event `self.BP_StarPointedShoot`
  ;[1 1 1] Camera Pointed Shoot Movement
  (bind (_direction _fiedlofview _z_camera) (`Timeline|PointedShoot` :!via `PlayFromStart` :!label _label)
    (:`Update`
      (`CameraComponent.SetFieldOfView` (`self.Camera`) _fiedlofview)
      (`SceneComponent.K2_SetRelativeLocation` (`self.Camera`) (`KismetMathLibrary.MakeVector` 0.0 -3.0 _z_camera) false false))))

(event `self.BP_EndPointedShoot`
  ;[1 1 1] Camera Pointed Shoot Movement
  (goto _label :!via `Stop`))

(event `self.BP_StarCameraSprint`
  (bind (_camerarotationwithpawn_roll _camerarotationwithpawn_pitch _camerarotationwithpawn_yaw) (`KismetMathLibrary.BreakRotator` (`self.CameraRotationWithPawn`)))
  ;[1 1 1] Camera Sprint Movement
  (`|ExecutionSequence`
    (:`then_0`
      (bind (_direction _camera_y_movement) (`Timeline|Camera1Movement` :!label _label_2)
        (:`Update`
          (`SceneComponent.K2_SetRelativeLocation` (`self.Camera`) (`KismetMathLibrary.MakeVector` 0.0 _camera_y_movement (stale _camera_z_movement)) false false :!label _label_3)
          (`SceneComponent.K2_SetRelativeRotation` (`self.Camera`) (`KismetMathLibrary.MakeRotator` _camerarotationwithpawn_roll _camerarotationwithpawn_pitch (+ _camerarotationwithpawn_yaw (stale _camera_rotation_z))) false false))))
    (:`then_1`
      (bind (_direction_2 _camera_z_movement _camera_rotation_z) (`Timeline|Camera2Movement` :!label _label_4)
        (:`Update`
          (goto _label_3))))))

(event `self.BP_StarAttackUltimate`
  (bind (_camerarotationwithpawn_roll _camerarotationwithpawn_pitch _camerarotationwithpawn_yaw) (`KismetMathLibrary.BreakRotator` (`self.CameraRotationWithPawn`)))
  ;[1 1 1] StarJumpAttackUltimate
  (set `CameraComponent.bUsePawnControlRotation` false (`self.Camera`))
  (bind (_direction _camera_z_location _camera_y_rotation _springarm_y) (`Timeline|Timeline_7` :!via `PlayFromStart`)
    (:`Update`
      (`SceneComponent.K2_SetRelativeLocationAndRotation` (`self.Camera`) (`KismetMathLibrary.MakeVector` 0.0 -3.0 _camera_z_location) (`KismetMathLibrary.MakeRotator` _camerarotationwithpawn_roll (+ _camerarotationwithpawn_pitch _camera_y_rotation) _camerarotationwithpawn_yaw) false false)
      (`SceneComponent.K2_SetRelativeRotation` (`self.SpringArm`) (`KismetMathLibrary.MakeRotator` 0.0 _springarm_y) false false))
    (:`Finished`
      (set `CameraComponent.bUsePawnControlRotation` true (`self.Camera`) :!label _label_5))))

(event `self.SetScoopVisibility`
  (params (Visibilty :type Boolean))
  ;[1 1 1] ScoopVisibility
  (`SceneComponent.SetVisibility` (`self.ScoopRocket`) Visibilty false)
  (`SceneComponent.SetVisibility` (`self.SceneCaptureComponent2D`) Visibilty false)
  (`SceneComponent.SetVisibility` (`self.Layer2`) Visibilty false)
  (`SceneComponent.SetVisibility` (`self.Layer3`) Visibilty false)
  (`SceneComponent.SetVisibility` (`self.Layer4`) Visibilty false)
  (`SceneComponent.SetVisibility` (`self.Layer1`) Visibilty false))

(event `self.BP_EndCameraSprint`
  ;[1 1 1] Camera Sprint Movement
  (`|ExecutionSequence`
    (:`then_0`
      (goto _label_2 :!via `Stop`))
    (:`then_1`
      (goto _label_4 :!via `Stop`))))

(event `self.BP_EndAttackUltimate`
  (bind (_camerarotationwithpawn_roll _camerarotationwithpawn_pitch _camerarotationwithpawn_yaw) (`KismetMathLibrary.BreakRotator` (`self.CameraRotationWithPawn`)))
  ;[1 1 1] StarJumpAttackUltimate
  (set `CameraComponent.bUsePawnControlRotation` false (`self.Camera`))
  (bind (_direction _camera_z_location _camera_y_rotation) (`Timeline|Timeline_8` :!via `PlayFromStart`)
    (:`Update`
      (`SceneComponent.K2_SetRelativeLocationAndRotation` (`self.Camera`) (`KismetMathLibrary.MakeVector` 0.0 -3.0 _camera_z_location) (`KismetMathLibrary.MakeRotator` _camerarotationwithpawn_roll (+ _camerarotationwithpawn_pitch _camera_y_rotation) _camerarotationwithpawn_yaw) false false))
    (:`Finished`
      (goto _label_5))))

(event `self.BP_StarUnderShoot`
  ;[1 1 1] Camera Under Shoot Movement
  (bind (_direction _camera_y _z_camera) (`Timeline|Timeline_2` :!via `PlayFromStart` :!label _label_6)
    (:`Update`
      (`SceneComponent.K2_SetRelativeLocation` (`self.Camera`) (`KismetMathLibrary.MakeVector` 0.0 _camera_y _z_camera) false false))))

(event `self.BP_EndUnderShoot`
  ;[1 1 1] Camera Under Shoot Movement
  (goto _label_6 :!via `Stop`))

(event `self.BP_StarCameraPointed`
  ;[1 1 1] Camera Pointed Movement
  (bind (_direction _fiedlofview _armlocationz _armlocationy) (`Timeline|Timeline_0` :!via `PlayFromStart` :!label _label_7)
    (:`Update`
      (`SceneComponent.K2_SetRelativeLocation` (`self.Arms`) (`KismetMathLibrary.MakeVector` 1.0 _armlocationy _armlocationz) false false)
      (`CameraComponent.SetFieldOfView` (`self.Camera`) _fiedlofview))))

(event `self.BP_Death`
  ;[1 1 1] Death
  (`KismetSystemLibrary.PrintString` "Tas rigus mortis xDXxdxdxdXD" true true (struct :`R` 0.05725 :`B` 1.0 :`A` 1.0) 20.0))

(event `self.BP_EndCameraPointed`
  ;[1 1 1] Camera Pointed Movement
  (goto _label_7 :!via `Reverse`))

(event `self.BP_EndMovilityUltimate`
  (bind (_camerarotationwithpawn_roll _camerarotationwithpawn_pitch _camerarotationwithpawn_yaw) (`KismetMathLibrary.BreakRotator` (`self.CameraRotationWithPawn`)))
  ;[1 1 1] Movility Ultimate
  (set `CameraComponent.bUsePawnControlRotation` true (`self.Camera`))
  (bind (_direction _camera_z_movement _camera_rotation_z _camera_rotation_y) (`Timeline|Timeline_10` :!via `Stop` :!label _label_8)
    (:`Update`
      (`SceneComponent.K2_SetRelativeLocationAndRotation` (`self.Camera`) (`KismetMathLibrary.MakeVector` 0.0 -3.0 _camera_z_movement) (`KismetMathLibrary.MakeRotator` _camerarotationwithpawn_roll (+ _camerarotationwithpawn_pitch _camera_rotation_y) (+ _camerarotationwithpawn_yaw _camera_rotation_z)) false false))))

(event `self.BP_StarGrenadeLauncher`
  (bind (_camerarotationwithpawn_roll _camerarotationwithpawn_pitch _camerarotationwithpawn_yaw) (`KismetMathLibrary.BreakRotator` (`self.CameraRotationWithPawn`)))
  ;[1 1 1] Grenade Camera
  (bind (_direction _camerarotation_z _camera_rotation__y) (`Timeline|Timeline_3` :!via `PlayFromStart`)
    (:`Update`
      (`SceneComponent.K2_SetRelativeRotation` (`self.Camera`) (`KismetMathLibrary.MakeRotator` _camerarotationwithpawn_roll (+ _camerarotationwithpawn_pitch _camera_rotation__y) (+ _camerarotationwithpawn_yaw _camerarotation_z)) false false))
    (:`Finished`
      (set `CameraComponent.bUsePawnControlRotation` true (`self.Camera`)))))

(event `self.BP_StartMovilityUltimate`
  (`|ExecutionSequence`
    (:`then_0`
      ;[1 1 1] Movility Ultimate
      (set `CameraComponent.bUsePawnControlRotation` false (`self.Camera`))
      (goto _label_8))))

(event `self.BP_StarCameraJump`
  ;[1 1 1] Jump Camera Logic
  (if (`self.bIsAttackUltimate`)
    (`KismetSystemLibrary.Delay` 2.0)
    (set `CharacterMovementComponent.GravityScale` 0.05 (`self.CharacterMovement`))))

(event `self.BP_EndGrenadeLauncher`
  ;[1 1 1] Grenade Camera
)

(event `self.BP_EndCameraJump`
  ;[1 1 1] Jump Camera Logic
  (set `self.bIsDelay` false))

(event `self.BP_StarMeleeAttack`
  (bind (_camerarotationwithpawn_roll _camerarotationwithpawn_pitch _camerarotationwithpawn_yaw) (`KismetMathLibrary.BreakRotator` (`self.CameraRotationWithPawn`)))
  (bind (_camerarotationwithpawn_roll_2 _camerarotationwithpawn_pitch_2 _camerarotationwithpawn_yaw_2) (`KismetMathLibrary.BreakRotator` (`self.CameraRotationWithPawn`)))
  ;[1 1 1] Melee Attack Movement
  (if (`|EnumInequality` (`self.MovementStatus`) "EMS_Sprinting")
    (bind (_direction _camera_location__x _camera_rotation_z _camera_y_rotation) (`Timeline|Timeline_4` :!via `PlayFromStart`)
      (:`Update`
        (`SceneComponent.K2_SetRelativeLocationAndRotation` (`self.Camera`) (`KismetMathLibrary.MakeVector` _camera_location__x -3.0 60.0) (`KismetMathLibrary.MakeRotator` _camerarotationwithpawn_roll_2 (+ _camerarotationwithpawn_pitch_2 _camera_y_rotation) (+ _camera_rotation_z _camerarotationwithpawn_yaw_2)) false false))
      (:`Finished`
        (set `CameraComponent.bUsePawnControlRotation` true (`self.Camera`) :!label _label_9)))
    (else
      (bind (_direction_2 _camera_location__x_2 _camera_rotation_z_2 _camera_y_rotation_2) (`Timeline|Timeline_5` :!via `PlayFromStart`)
        (:`Update`
          (`SceneComponent.K2_SetRelativeLocationAndRotation` (`self.Camera`) (0.0 -3.0 60.0) (`KismetMathLibrary.MakeRotator` _camerarotationwithpawn_roll (+ _camerarotationwithpawn_pitch _camera_rotation_z_2) (+ _camera_y_rotation_2 _camerarotationwithpawn_yaw)) false false))
        (:`Finished`
          (goto _label_9))))))

(event `self.BP_EndMeleeAttack`
  ;[1 1 1] Melee Attack Movement
)

(event `self.BP_StarReload`
  (bind (_camerarotationwithpawn_roll _camerarotationwithpawn_pitch _camerarotationwithpawn_yaw) (`KismetMathLibrary.BreakRotator` (`self.CameraRotationWithPawn`)))
  ;[1 1 1] Reload Camera Movement
  (bind (_direction _arms_z _camera_rotation_z _camera_y_rotation) (`Timeline|Timeline_6` :!via `PlayFromStart`)
    (:`Update`
      (`SceneComponent.K2_SetRelativeRotation` (`self.Camera`) (`KismetMathLibrary.MakeRotator` _camerarotationwithpawn_roll (+ _camerarotationwithpawn_pitch _camera_y_rotation) (+ _camerarotationwithpawn_yaw _camera_rotation_z)) false false)
      (`SceneComponent.K2_SetRelativeRotation` (`self.SpringArm`) (`KismetMathLibrary.MakeRotator` 0.0 0.0 _arms_z) false false))
    (:`Finished`
      (set `CameraComponent.bUsePawnControlRotation` true (`self.Camera`)))))

(event `self.BP_EndReload`
  ;[1 1 1] Reload Camera Movement
)

(fn `UserConstructionScript`)