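; Enemy pawn Blueprint that reacts to taking damage and shuts off its controller when health runs out.
; On BeginPlay it binds to its own any-damage event, which prints the ORHealth component's current health on each hit.
; At zero health or below, a DoOnce unpossesses the pawn; it is not destroyed, as the DestroyActor node is unconnected.
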(event `self.ReceiveTick`
  (params (DeltaSeconds :type "Float (single-precision)")))

(event `self.ReceiveBeginPlay`
  (add `self.OnTakeAnyDamage` (delegate `OnTakeAnyDamage_Event_0`)))

(event `OnTakeAnyDamage_Event_0` :!signature `self.OnTakeAnyDamage`
  (params (DamagedActor :type "Actor Object Reference") (Damage :type "Float (double-precision)") (DamageType :type "DamageType Object Reference") (InstigatedBy :type "Controller Object Reference") (DamageCauser :type "Actor Object Reference"))
  (bind _currenthealth (`OR_HealthComponent.CurrentHealth` (`self.OR_Health`)))
  (`KismetSystemLibrary.PrintString` (`KismetStringLibrary.Conv_DoubleToString` _currenthealth))
  (if (<= _currenthealth 0.0)
    (`/Engine/EditorBlueprintResources/StandardMacros.DoOnce` false
      (:`Completed`
        (`Controller.UnPossess` (`self.GetController`))))))

(fn `UserConstructionScript`)